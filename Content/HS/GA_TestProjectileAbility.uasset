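; Test gameplay ability that spawns a BP_Projectile when activated, then ends immediately.
; It aims with the ReplicatedRotation from the HsPlayerState found through the avatar's instigator controller.
; If that cast fails, it falls back to the avatar actor's own rotation.
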(event `self.K2_ActivateAbility`
  (bind _ashs_player_state (cast `HsPlayerState` (`Controller.PlayerState` (`Pawn.GetController` (`Actor.Instigator` (`self.GetAvatarActorFromActorInfo`)))))
    (:`then`
      (`self.SpawnProjectile` "/Game/HS/BP_Projectile.BP_Projectile_C" (`HsPlayerState.ReplicatedRotation` _ashs_player_state)))
    (:`CastFailed`
      (`self.SpawnProjectile` "/Game/HS/BP_Projectile.BP_Projectile_C" (`Actor.K2_GetActorRotation` (`self.GetAvatarActorFromActorInfo`)))))
  (`self.K2_EndAbility`))